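; BP_P38 is a player-controlled P38 pawn that constantly moves forward, steers in roll and pitch, and fires rockets.
; Tick feeds MoveSpeed into AddMovementInput along the forward vector, Boost raises it while held, and the Roll and Pitch axes apply frame-time-scaled local rotation.
; Fire spawns BP_Rocket at the Body's RocketSpawn socket.
; The MoveForward function and extra rotation nodes are unconnected leftovers that never run.
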(event `self.ReceiveTick`
  (params (DeltaSeconds :type "Float (single-precision)"))
  ; Move
  (`self.AddMovementInput` (`self.GetActorForwardVector`) (`self.MoveSpeed`)))

(event `InputAxis|Roll`
  (params (AxisValue :type "Float (single-precision)"))
  ; Input Rotate
  (`self.K2_AddActorLocalRotation` (`KismetMathLibrary.MakeRotator` (* AxisValue (`self.RotationSpeed`) (`GameplayStatics.GetWorldDeltaSeconds`)))))

(event `InputAxis|Pitch`
  (params (AxisValue :type "Float (single-precision)"))
  ; Input Rotate
  (`self.K2_AddActorLocalRotation` (`KismetMathLibrary.MakeRotator` 0.0 (* AxisValue (`self.RotationSpeed`) (`GameplayStatics.GetWorldDeltaSeconds`)))))

(event `InputAction|Boost`
  (params (Key :type "Key Structure"))
  ; Boost
  (:`Pressed`
    (set `self.MoveSpeed` 1.0))
  (:`Released`
    (set `self.MoveSpeed` 0.5)))

(event `InputAction|Fire`
  (params (Key :type "Key Structure"))
  ; Fire
  (:`Pressed`
    (`|SpawnActorFromClass` "/Game/P38/Blueprints/BP_Rocket.BP_Rocket_C" (`SceneComponent.GetSocketTransform` (`self.Body`) "RocketSpawn" "RTS_World") "Undefined" "MultiplyWithRoot" null null)))

(fn `MoveForward`
  (params (B :type "Float (single-precision)"))
  (`self.AddMovementInput` (* (`self.GetActorForwardVector`) B (`self.MoveSpeed`))))

(fn `UserConstructionScript`)